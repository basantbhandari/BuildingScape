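; Openable door actor that swings open and closed in response to OnOpen and OnClose events from OpenDoor.
; It stores its rotation at BeginPlay, then the Door_Swin timeline adds an animated yaw angle to it and rotates the whole actor.
; OnOpen plays the timeline and OnClose reverses it.
; An event track on the timeline plays a lock sound at the door's location.
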(event OnClose(OpenDoor)
  (bind _openangle (Timeline|Door_Swin Reverse)
    (:Update
      (Transformation|SetActorRotation (Math|Rotator|CombineRotators (Math|Rotator|MakeRotator 0.0 0.0 _openangle) (Variables|Default|GetNew%20Rotation))))
    (:Sound%20Track
      (Audio|PlaySoundatLocation "/Game/Audio/door_lock_wav.door_lock_wav" (Transformation|GetActorLocation) "0, 0, 0" 1.0 1.0 0.0 0 0 0))))

(event OnOpen(OpenDoor)
  (bind _openangle (Timeline|Door_Swin Play)
    (:Update
      (Transformation|SetActorRotation (Math|Rotator|CombineRotators (Math|Rotator|MakeRotator 0.0 0.0 _openangle) (Variables|Default|GetNew%20Rotation))))
    (:Sound%20Track
      (Audio|PlaySoundatLocation "/Game/Audio/door_lock_wav.door_lock_wav" (Transformation|GetActorLocation) "0, 0, 0" 1.0 1.0 0.0 0 0 0))))

(event EventBeginPlay
  (Variables|Default|SetNew%20Rotation (Transformation|GetActorRotation)))

(fn ConstructionScript)